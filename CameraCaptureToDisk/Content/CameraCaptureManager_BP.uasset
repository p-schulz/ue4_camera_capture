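; Camera capture manager Blueprint that configures a named sensor on a target vehicle, all in its construction script.
; It lists the vehicle's child actors into SensorsAvailable and casts the one matching SensorName to a SceneCapture2D.
; CaptureType selects Camera, Semantic Segmentation, Depth or Radar; all toggle per-frame capture through Active.
; Only Camera also applies field of view and enables ray tracing; the event graph is unused.
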(event EventBeginPlay)

(event Collision|EventActorBeginOverlap
  (params (OtherActor :type Actor%20Object%20Reference)))

(event EventTick
  (params (DeltaSeconds :type Float%20%28single-precision%29)))

(fn ConstructionScript
  (bind _targetvehicle (Variables|Capture|GetTargetVehicle))
  (bind _active (Variables|Capture|GetActive))
  (bind _childactors (Actor|GetAllChildActors _targetvehicle false))
  (Utilities|Array|Clear (Variables|Capture|GetSensorsAvailable))
  (for _index (range 0 (Utilities|Array|LastIndex _childactors))
    (Utilities|Array|Add (Variables|Capture|GetSensorsAvailable) (Utilities|GetDisplayName (Utilities|Array|Get(acopy) _childactors _index)))
    (if (Utilities|Enum|Equal(Enum) (Utilities|GetDisplayName (Utilities|Array|Get(acopy) _childactors _index)) (Variables|Capture|GetSensorName))
      (switch Utilities|FlowControl|Switch|SwitchonCaptureType (Variables|Capture|GetCaptureType)
        (:NewEnumerator0
          (bind _asscene_capture_2d (Utilities|Casting|CastToSceneCapture2D (Utilities|Array|Get(acopy) _childactors _index)))
          (bind _output_get (Variables|Default|SetCaptureComponent _asscene_capture_2d))
          (Variables|/Script/Engine.SceneCaptureComponent2D|SetFOVAngle (Variables|/Script/Engine.SceneCapture2D|GetCaptureComponent2D _output_get) (Variables|Default|GetField%20Of%20View))
          (Variables|/Script/Engine.SceneCaptureComponent|SetbCaptureEveryFrame (Variables|/Script/Engine.SceneCapture2D|GetCaptureComponent2D _output_get) _active)
          (Variables|/Script/Engine.SceneCaptureComponent|SetbUseRayTracingIfEnabled (Variables|/Script/Engine.SceneCapture2D|GetCaptureComponent2D _output_get) true))
        (:NewEnumerator1
          (bind _asscene_capture_2d_2 (Utilities|Casting|CastToSceneCapture2D (Utilities|Array|Get(acopy) _childactors _index)))
          (bind _output_get_2 (Variables|Default|SetCaptureComponent _asscene_capture_2d_2))
          (Variables|/Script/Engine.SceneCaptureComponent|SetbCaptureEveryFrame (Variables|/Script/Engine.SceneCapture2D|GetCaptureComponent2D _output_get_2) _active))
        (:NewEnumerator2
          (bind _asscene_capture_2d_3 (Utilities|Casting|CastToSceneCapture2D (Utilities|Array|Get(acopy) _childactors _index)))
          (bind _output_get_3 (Variables|Default|SetCaptureComponent _asscene_capture_2d_3))
          (Variables|/Script/Engine.SceneCaptureComponent|SetbCaptureEveryFrame (Variables|/Script/Engine.SceneCapture2D|GetCaptureComponent2D _output_get_3) _active))
        (:NewEnumerator3
          (bind _asscene_capture_2d_4 (Utilities|Casting|CastToSceneCapture2D (Utilities|Array|Get(acopy) _childactors _index)))
          (bind _output_get_4 (Variables|Default|SetCaptureComponent _asscene_capture_2d_4))
          (Variables|/Script/Engine.SceneCaptureComponent|SetbCaptureEveryFrame (Variables|/Script/Engine.SceneCapture2D|GetCaptureComponent2D _output_get_4) _active))))))